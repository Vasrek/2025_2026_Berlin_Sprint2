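; AI pawn that chases the player on sight and searches outward once the player is lost.
; AI Perception updates toggle CanSeePlayer, starting either a chase toward the player or a patrol around the stimulus location.
; Both behaviors are self-recalling AIMoveTo loops that pause briefly after each successful move.
; Patrol picks random reachable points, doubling its search radius after each arrival; chasing resets that radius.
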(event OnTargetPerceptionUpdated(AIPerception)
  (params (Actor :type Actor%20Object%20Reference) (Stimulus :type AI%20Stimulus%20Structure))
  (if (.bsuccessfullysensed Stimulus)
    (Variables|Default|SetbCanSeePlayer? true)
    (CallFunction|ChasePlayer)
    (else
      (Variables|Default|SetbCanSeePlayer? false)
      (CallFunction|Patrol (.stimuluslocation Stimulus)))))

(event Custom|ChasePlayer
  (if (Variables|Default|GetbCanSeePlayer?)
    (Variables|Default|SetRadiusOrigin 3e+02)
    (AI|AIMoveTo self "0, 0, 0" (Game|GetPlayerCharacter 0) 1e+02 false
      (:OnSuccess
        (Utilities|FlowControl|Delay 2.0)
        (CallFunction|ChasePlayer)))))

(event Custom|Patrol
  (params (Origin :type Vector%20%28by%20ref%29))
  (if (Variables|Default|GetbCanSeePlayer?)
    (CallFunction|ChasePlayer)
    (else
      (AI|AIMoveTo self (.RandomLocation (AI|Navigation|GetRandomReachablePointinRadius Origin (Variables|Default|GetRadiusOrigin) 0 0)) 0 1e+02 false
        (:OnSuccess
          (Utilities|FlowControl|Delay 2.0)
          (Variables|Default|SetRadiusOrigin (* (Variables|Default|GetRadiusOrigin) 2.0))
          (CallFunction|Patrol Origin))))))

(fn ConstructionScript)